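; Elevator actor whose platform moves up and down continuously from BeginPlay, with no trigger or stop logic.
; TurnElevatorOn starts the Raise timeline, whose completion calls ElevatorLower to play the Lower timeline in reverse, which then calls ElevatorRaise again.
; Both timelines drive the Platform component's relative Z from a float track scaled by 100.
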(event `self.ReceiveBeginPlay`
  (`self.TurnElevatorOn`))

(event `ElevatorRaise`
  (bind (_direction _raiseelevatorvalue) (`Timeline|Raise` :!via `PlayFromStart`)
    (:`Update`
      (`SceneComponent.K2_SetRelativeLocation` (`self.Platform`) (`KismetMathLibrary.MakeVector` 0.0 0.0 (* _raiseelevatorvalue 100.0)) false false))
    (:`Finished`
      (`self.ElevatorLower`))))

(event `ElevatorLower`
  (bind (_direction _raiseelevatorvalue) (`Timeline|Lower` :!via `ReverseFromEnd`)
    (:`Update`
      (`SceneComponent.K2_SetRelativeLocation` (`self.Platform`) (`KismetMathLibrary.MakeVector` 0.0 0.0 (* _raiseelevatorvalue 100.0)) false false))
    (:`Finished`
      (`self.ElevatorRaise`))))

(event `TurnElevatorOn`
  (`self.ElevatorRaise`))

(fn `UserConstructionScript`)