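; BP_Door is a sliding door that opens for the ThirdPersonCharacter when it is not locked.
; Entering the CheckForPlayerTrigger volume plays the DoorSlide timeline, moving InnerDoorPiece along its relative Z.
; Leaving it plays a separate DoorReturn timeline in reverse from the end to close the door.
; Tick refreshes LockedText every frame to show the IsDoorLocked state, which also gates both overlap responses.
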(event `self.ReceiveTick`
  (params (DeltaSeconds :type "Float (single-precision)"))
  (if (`self.IsDoorLocked`)
    (`TextRenderComponent.K2_SetText` (`self.LockedText`) "Looked")
    (else
      (`TextRenderComponent.K2_SetText` (`self.LockedText`) "Unlooked"))))

(event `self.CheckForPlayerTrigger.OnComponentBeginOverlap`
  (params (OverlappedComponent :type "PrimitiveComponent Object Reference") (OtherActor :type "Actor Object Reference") (OtherComp :type "PrimitiveComponent Object Reference") (OtherBodyIndex :type Integer) (bFromSweep :type Boolean) (SweepResult :type "HitResult Structure (by ref)"))
  (cast `/Game/ThirdPersonBP/Blueprints/ThirdPersonCharacter` OtherActor)
  (if (not (`self.IsDoorLocked`))
    (`KismetSystemLibrary.PrintString` "Door")
    (bind (_direction _slimeamount) (`Timeline|DoorSlide` :!via `PlayFromStart`)
      (:`Update`
        (`SceneComponent.K2_SetRelativeLocation` (`self.InnerDoorPiece`) (`KismetMathLibrary.MakeVector` 0.0 0.0 (* _slimeamount 63.0)) false false)))))

(event `self.CheckForPlayerTrigger.OnComponentEndOverlap`
  (params (OverlappedComponent :type "PrimitiveComponent Object Reference") (OtherActor :type "Actor Object Reference") (OtherComp :type "PrimitiveComponent Object Reference") (OtherBodyIndex :type Integer))
  (cast `/Game/ThirdPersonBP/Blueprints/ThirdPersonCharacter` OtherActor)
  (if (not (`self.IsDoorLocked`))
    (bind (_direction _slimeamount) (`Timeline|DoorReturn` :!via `ReverseFromEnd`)
      (:`Update`
        (`SceneComponent.K2_SetRelativeLocation` (`self.InnerDoorPiece`) (`KismetMathLibrary.MakeVector` 0.0 0.0 (* _slimeamount 63.0)) false false)))))

(fn `UserConstructionScript`)